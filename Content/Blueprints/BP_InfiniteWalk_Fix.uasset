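; Actor that walks a skeletal mesh along a spline repeatedly, driven by the BP_Player StartCheck and ResetCheck flags.
; Tick either resets it to the first spline point or runs Walking, which waits out a one-time start delay.
; Walking moves it by elapsed time times speed, with height and -90 yaw offsets.
; At the last point, closed splines restart after a Delay, while open ones snap back to the start.
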(event `self.ReceiveTick`
  (params (DeltaSeconds :type "Float (single-precision)"))
  (bind _asbp_player (cast `/Game/Blueprints/BP_Player` (`GameplayStatics.GetPlayerPawn` 0)))
  (`/Engine/EditorBlueprintResources/StandardMacros.IsValid` _asbp_player
    (:`Is Valid`
      (if (`/Game/Blueprints/BP_Player.ResetCheck` _asbp_player)
        (`self.ResetTransform`)
        (elif (`/Game/Blueprints/BP_Player.StartCheck` _asbp_player)
          (`self.Walking`))))))

(event `Walking`
  (bind _spline (`self.Spline`))
  (bind _startdelay (`self.StartDelay`))
  (bind _spline_2 (`self.Spline`))
  (bind (_returnvalue_roll _returnvalue_pitch _returnvalue_yaw) (`KismetMathLibrary.BreakRotator` (`SplineComponent.GetRotationAtSplinePoint` _spline_2 0 "World")))
  (if (!= _startdelay 0.0)
    (bind _output_get (set `self.StartDelayTime` (+ (`self.StartDelayTime`) (`GameplayStatics.GetWorldDeltaSeconds`))))
    (if (>= _output_get _startdelay)
      (set `self.StartDelay` 0.0)
      (set `SkeletalMeshComponent.GlobalAnimRateScale` (`self.AnimPlayRate`) (`self.SkeletalMesh`) :!label _label)
      (set `self.Time` (+ (`self.Time`) (`GameplayStatics.GetWorldDeltaSeconds`)))
      (`self.SetWorldTransform`)
      (if (== (`SplineComponent.GetLocationAtSplinePoint` _spline (- (`SplineComponent.GetNumberOfSplinePoints` _spline) 1) "World") (`SceneComponent.K2_GetComponentLocation` (`self.SkeletalMesh`)) :`ErrorTolerance` (`self.MeshHeight`))
        (if (`SplineComponent.IsClosedLoop` (`self.Spline`))
          (`self.SetWorldTransform`)
          (`KismetSystemLibrary.Delay` (`self.LoopDelayDuration`))
          (set `self.Time` 0.0)
          (else
            (`SceneComponent.K2_SetWorldTransform` (`self.SkeletalMesh`) (`KismetMathLibrary.MakeTransform` (`SplineComponent.GetLocationAtSplinePoint` _spline_2 0 "World") (`KismetMathLibrary.MakeRotator` _returnvalue_roll _returnvalue_pitch (+ _returnvalue_yaw -90.0))) false false)
            (set `self.Time` 0.0)))
        (set `self.StartDelayTime` 0.0)))
    (else
      (goto _label))))

(fn `ResetTransform`
  (bind _spline (`self.Spline`))
  (bind (_returnvalue_roll _returnvalue_pitch _returnvalue_yaw) (`KismetMathLibrary.BreakRotator` (`SplineComponent.GetRotationAtSplinePoint` _spline 0 "World")))
  (`SceneComponent.K2_SetWorldTransform` (`self.SkeletalMesh`) (`KismetMathLibrary.MakeTransform` (`SplineComponent.GetLocationAtSplinePoint` _spline 0 "World") (`KismetMathLibrary.MakeRotator` _returnvalue_roll _returnvalue_pitch (+ _returnvalue_yaw -90.0))) false false)
  (set `self.Time` 0.0)
  (set `self.StartDelayTime` 0.0))

(fn `SetWorldTransform`
  (bind _spline (`self.Spline`))
  (bind _returnvalue (* (`self.Time`) (`self.WalkSpeed`)))
  (bind (_returnvalue_x _returnvalue_y _returnvalue_z) (`KismetMathLibrary.BreakVector` (`SplineComponent.GetLocationAtDistanceAlongSpline` _spline _returnvalue "World")))
  (bind (_returnvalue_roll _returnvalue_pitch _returnvalue_yaw) (`KismetMathLibrary.BreakRotator` (`SplineComponent.GetRotationAtDistanceAlongSpline` _spline _returnvalue "World")))
  (`SceneComponent.K2_SetWorldTransform` (`self.SkeletalMesh`) (`KismetMathLibrary.MakeTransform` (`KismetMathLibrary.MakeVector` _returnvalue_x _returnvalue_y (+ _returnvalue_z (`self.MeshHeight`))) (`KismetMathLibrary.MakeRotator` _returnvalue_roll _returnvalue_pitch (+ _returnvalue_yaw -90.0))) false false)
  (return))

(fn `UserConstructionScript`
  (set `self.WalkSpeed` (`self.WalkSpeed`))
  (set `self.MeshHeight` (`self.MeshHeight`))
  (set `SkeletalMeshComponent.GlobalAnimRateScale` (`self.AnimPlayRate`) (`self.SkeletalMesh`))
  (set `self.LoopDelayDuration` (`self.LoopDelayDuration`)))