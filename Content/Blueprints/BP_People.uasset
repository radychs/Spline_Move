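; BP_People is an actor that walks a skeletal mesh along its spline, likely as a moving background pedestrian.
; On BeginPlay a timeline scales spline length into a distance, and each update places the mesh there in world space, using only the spline's yaw with a mesh-facing offset.
; When the timeline finishes, it restarts only if the spline's StationaryEndpoints flag is set.
; A delayed restart and a time-based speed calculation are left unconnected.
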(event `self.ReceiveTick`
  (params (DeltaSeconds :type "Float (single-precision)")))

(event `self.ReceiveBeginPlay`
  (bind _spline (`self.Spline`))
  (bind _bstationaryendpoints (`SplineComponent.bStationaryEndpoints` _spline))
  (bind (_direction `_새_트랙_0`) (`Timeline|타임라인_0` :!via `PlayFromStart` :!label _label)
    (:`Update`
      (bind _returnvalue (* (`SplineComponent.GetSplineLength` _spline) `_새_트랙_0`))
      (bind (_returnvalue_roll _returnvalue_pitch _returnvalue_yaw) (`KismetMathLibrary.BreakRotator` (`SplineComponent.GetRotationAtDistanceAlongSpline` _spline _returnvalue "World")))
      (`SceneComponent.K2_SetWorldTransform` (`self.SkeletalMesh`) (`KismetMathLibrary.MakeTransform` (`SplineComponent.GetLocationAtDistanceAlongSpline` _spline _returnvalue "World") (`KismetMathLibrary.MakeRotator` 0.0 0.0 (+ _returnvalue_yaw -90.0))) false false))
    (:`Finished`
      (set `self.Stationary Endpoints` _bstationaryendpoints)
      (if _bstationaryendpoints
        (goto _label :!via `PlayFromStart`)))))

(fn `UserConstructionScript`)