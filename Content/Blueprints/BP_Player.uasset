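; BP_Player is a player-controlled pawn with free-look rotation, directional movement and vertical travel.
; Forward and right axes feed AddMovementInput along actor vectors, while look axes pitch and yaw the root and UP/Down axes shift it along world Z.
; Key 1 toggles StartCheck via FlipFlop, and key 2 holds ResetCheck true until released using a DoOnce; neither flag is read in these graphs.
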(event `Key|Two`
  (params (Key :type "Key Structure"))
  (:`Pressed`
    (`/Engine/EditorBlueprintResources/StandardMacros.DoOnce` false :!label _label
      (:`Completed`
        (set `self.ResetCheck` true))))
  (:`Released`
    (set `self.ResetCheck` false)
    (goto _label :!via `Reset`)))

(event `Key|One`
  (params (Key :type "Key Structure"))
  (:`Pressed`
    (`/Engine/EditorBlueprintResources/StandardMacros.FlipFlop`
      (:`A`
        (set `self.StartCheck` true))
      (:`B`
        (set `self.StartCheck` false)))))

(event `InputAxis|UP`
  (params (AxisValue :type "Float (single-precision)"))
  (`SceneComponent.K2_AddWorldTransform` (`self.DefaultSceneRoot`) (`KismetMathLibrary.MakeTransform` (`KismetMathLibrary.MakeVector` 0.0 0.0 (* AxisValue 5.0))) false false))

(event `InputAxis|LookUp`
  (params (AxisValue :type "Float (single-precision)"))
  (`SceneComponent.K2_AddRelativeRotation` (`self.DefaultSceneRoot`) (`KismetMathLibrary.MakeRotator` 0.0 AxisValue) false false))

(event `InputAxis|LookUpRate`
  (params (AxisValue :type "Float (single-precision)"))
  (`SceneComponent.K2_AddRelativeRotation` (`self.DefaultSceneRoot`) (`KismetMathLibrary.MakeRotator` 0.0 0.0 AxisValue) false false))

(event `InputAxis|Down`
  (params (AxisValue :type "Float (single-precision)"))
  (`SceneComponent.K2_AddWorldTransform` (`self.DefaultSceneRoot`) (`KismetMathLibrary.MakeTransform` (`KismetMathLibrary.MakeVector` 0.0 0.0 (* AxisValue 5.0))) false false))

(event `InputAxis|MoveForward`
  (params (AxisValue :type "Float (single-precision)"))
  (`self.AddMovementInput` self (`self.GetActorForwardVector` self) AxisValue false))

(event `InputAxis|MoveRight`
  (params (AxisValue :type "Float (single-precision)"))
  (`self.AddMovementInput` self (`self.GetActorRightVector` self) AxisValue false))

(fn `UserConstructionScript`)